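; Main menu actor that hosts the WBP_MainMenu widget and previews arcade and simulation ship meshes for the mode selector.
; Both ships start hidden; HandleModeSelector toggles their visibility and the looping of the ShipsMove timeline, which it plays when switched on.
; The timeline's SimulationAlpha vector drives ship rotation, with roll applied only to the simulation ship.
; Every tick, the widget component turns to face the player camera.
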(event `self.ReceiveBeginPlay`
  (set `/Game/Blueprint/Widget/WBP_MainMenu.BP_MainMenu` null self (cast `/Game/Blueprint/Widget/WBP_MainMenu` (`WidgetComponent.GetWidget` (`self.Widget`)) :!pure true))
  (`SceneComponent.SetVisibility` (`self.SM_ShipArcade`) false false)
  (`SceneComponent.SetVisibility` (`self.SM_ShipSimu`) false false))

(event `HandleModeSelector`
  (params (`On?` :type Boolean))
  (`TimelineComponent.SetLooping` (`self.shipsMove`) `On?`)
  (`SceneComponent.SetVisibility` (`self.SM_ShipArcade`) `On?` false)
  (`SceneComponent.SetVisibility` (`self.SM_ShipSimu`) `On?` false)
  (if `On?`
    (bind (_direction _simulationalpha) (`Timeline|shipsMove`)
      (:`Update`
        (bind _y (.y _simulationalpha))
        (bind _z (.z _simulationalpha))
        (`SceneComponent.K2_SetWorldRotation` (`self.SM_ShipSimu`) (`KismetMathLibrary.MakeRotator` (.x _simulationalpha) _y _z) false false)
        (`SceneComponent.K2_SetWorldRotation` (`self.SM_ShipArcade`) (`KismetMathLibrary.MakeRotator` 0.0 _y _z) false false)))))

(event `self.ReceiveTick`
  (params (DeltaSeconds :type "Float (single-precision)"))
  (`SceneComponent.K2_SetWorldRotation` (`self.Widget`) (`KismetMathLibrary.FindLookAtRotation` (`SceneComponent.K2_GetComponentLocation` (`self.Widget`)) (`PlayerCameraManager.GetCameraLocation` (`GameplayStatics.GetPlayerCameraManager` 0))) false false))

(fn `UserConstructionScript`)