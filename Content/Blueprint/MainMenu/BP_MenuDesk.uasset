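; Main menu desk with a rotating carousel of colored map meshes, spun by a hand swipe to choose a level.
; Construction spaces the meshes along a spline and tints each with a dynamic material.
; An overlapping hand's socket movement sets a swipe direction, which shifts MapIndex when overlap ends, and Tick eases the spline's yaw to match.
; ValidateLevel unloads the previous streamed level and loads the selected one hidden.
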(event `self.ReceiveBeginPlay`)

(event `self.ReceiveTick`
  (params (DeltaSeconds :type "Float (single-precision)"))
  (bind _spline (`self.Spline`))
  (`|ExecutionSequence`
    (:`then_0`
      (bind _arms (`self.Arms`)
        (:`then`
          (bind _returnvalue (`SceneComponent.GetSocketLocation` _arms (select `bool` (`self.RightHand`) :`false` (select `bool` (`self.LeftHand`) :`true` "IndexL" :!type "Name") :`true` "IndexR")))
          (bind _output_get (set `self.Velocity` (- (`self.PreviousLocation`) _returnvalue)))
          (set `self.PreviousLocation` _returnvalue)
          (bind _y (.y _output_get))
          (if (> (`KismetMathLibrary.Abs` _y) 2.0)
            (set `self.HandDirection` (`KismetMathLibrary.Clamp` (`KismetMathLibrary.Round` _y) -1 1))))
        (:`else`)))
    (:`then_1`
      (`SceneComponent.K2_SetRelativeRotation` _spline (`KismetMathLibrary.RInterpTo` (`SceneComponent.RelativeRotation` _spline) (`KismetMathLibrary.MakeRotator` 0.0 0.0 (+ (* (/ 360.0 (`KismetArrayLibrary.Array_Length` (`self.MapsMeshes`))) (`self.MapIndex`)) -37.5)) (`GameplayStatics.GetWorldDeltaSeconds`) 5.0) false false))))

(event `ValidateLevel`
  (bind _output (`|GetArrayItem` (`self.Level`) (`self.MapIndex`)))
  (bind _actuallevelloaded (`self.ActualLevelLoaded`)
    (:`then`
      (`GameplayStatics.UnloadStreamLevelBySoftObjectPtr` _actuallevelloaded))
    (:`else`
      _))
  (`GameplayStatics.LoadStreamLevelBySoftObjectPtr` _output)
  (set `self.ActualLevelLoaded` _output))

(event `self.Box.OnComponentBeginOverlap`
  (params (OverlappedComponent :type "PrimitiveComponent Object Reference") (OtherActor :type "Actor Object Reference") (OtherComp :type "PrimitiveComponent Object Reference") (OtherBodyIndex :type Integer) (bFromSweep :type Boolean) (SweepResult :type "HitResult Structure (by ref)"))
  (bind _asvrpawn (cast `` OtherActor))
  (bind _output_get (set `self.LeftHand` (`PrimitiveComponent.IsOverlappingActor` (`/Game/Blueprint/MainMenu/BP_MenuDesk.CapsuleL` _asvrpawn) self)))
  (if _output_get
    (`self.DeactiveInteractionMode` _asvrpawn :!label _label)
    (bind _arms (`/Game/Blueprint/MainMenu/BP_MenuDesk.Arms` _asvrpawn))
    (set `self.PreviousLocation` (`SceneComponent.K2_GetComponentLocation` _arms))
    (set `self.Arms` _arms)
    (else
      (bind _output_get_2 (set `self.RightHand` (`PrimitiveComponent.IsOverlappingActor` (`/Game/Blueprint/MainMenu/BP_MenuDesk.CapsuleR` _asvrpawn) self)))
      (if _output_get_2
        (goto _label)))))

(event `self.Box.OnComponentEndOverlap`
  (params (OverlappedComponent :type "PrimitiveComponent Object Reference") (OtherActor :type "Actor Object Reference") (OtherComp :type "PrimitiveComponent Object Reference") (OtherBodyIndex :type Integer))
  (if true
    (set `self.MapIndex` (+ (`self.MapIndex`) (`self.HandDirection`)))))

(fn `UserConstructionScript`
  (bind _array (`|MakeArray` (`self.BleuClair`) (`self.Jaune`) (`self.Rouge`) (`self.Violet`) (`self.Bleue`)))
  (set `self.MapsMeshes` _array)
  (for (_array_element _array_index) _array
    (bind _returnvalue (`PrimitiveComponent.CreateDynamicMaterialInstance` _array_element 0 null "None"))
    (`MaterialInstanceDynamic.SetVectorParameterValue` _returnvalue "Color" (select `int` _array_index :`0` (struct :`R` 1.0 :`A` 1.0) :`1` (struct :`R` 0.510729 :`G` 1.0 :`A` 1.0) :`2` (struct :`G` 0.965735 :`B` 1.0 :`A` 1.0) :`3` (struct :`G` 0.016063 :`B` 1.0 :`A` 1.0) :`4` (struct :`R` 0.905564 :`B` 1.0 :`A` 1.0) :!type "LinearColor Structure"))
    (`PrimitiveComponent.SetMaterial` _array_element 0 _returnvalue)
    (`SceneComponent.K2_SetWorldLocation` _array_element (`SplineComponent.GetLocationAtTime` (`self.Spline`) (/ (* 1.0 _array_index) (`KismetArrayLibrary.Array_Length` _array)) "World" false) false false)))