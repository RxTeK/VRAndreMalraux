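; VR level selector actor: a carousel of colored map meshes spaced along a spline, with text naming the current level.
; A hand swipe through the box, with a curl gesture, steps the wrapping map index using a dot product for direction.
; Tick smoothly rotates the spline to that index.
; It spawns and attaches an open-level button, and ValidateLevel has the spaceship load the selected map through a wormhole.
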(event `self.ReceiveBeginPlay`
  (bind _returnvalue (`|SpawnActorFromClass` "/Game/Blueprint/Command/Bp_ButtonOPenLevel.Bp_ButtonOPenLevel_C" (`KismetMathLibrary.MakeTransform` (0.0 0.0 0.0)) "AlwaysSpawn" "MultiplyWithRoot" null null))
  (bind _output_get (set `self.ButtonOpenLevelRef` _returnvalue))
  (set `/Game/Blueprint/Command/Bp_ButtonOPenLevel.LevelSelectorRef` null self _output_get)
  (`self.K2_AttachToComponent` _output_get (`self.Scene`) "None" "SnapToTarget" "SnapToTarget" "KeepRelative" true))

(event `self.ReceiveTick`
  (params (DeltaSeconds :type "Float (single-precision)"))
  (bind _spline (`self.Spline`))
  (`|ExecutionSequence`
    (:`then_0`
      (`SceneComponent.K2_SetRelativeRotation` _spline (`KismetMathLibrary.RInterpTo` (`SceneComponent.RelativeRotation` _spline) (`KismetMathLibrary.MakeRotator` 0.0 0.0 (+ (* (/ 360.0 (`KismetArrayLibrary.Array_Length` (`self.MapsMeshes`))) (* (`self.MapIndex`) -1)) 270.0)) (`GameplayStatics.GetWorldDeltaSeconds`) 5.0) false false))
    (:`then_1`
      (`TextRenderComponent.K2_SetText` (`self.TextRender`) (`KismetTextLibrary.Conv_StringToText` (`|GetArrayItem` (`self.LevelDebugName`) (`self.MapIndex`)))))))

(event `ValidateLevel`
  (`/Game/Blueprint/SpaceShip/BP_Spaceship.LoadLevelWithWormHole` (`self.SpaceShipRef`) (`self.MapIndex`) self))

(event `self.Box.OnComponentBeginOverlap`
  (params (OverlappedComponent :type "PrimitiveComponent Object Reference") (OtherActor :type "Actor Object Reference") (OtherComp :type "PrimitiveComponent Object Reference") (OtherBodyIndex :type Integer) (bFromSweep :type Boolean) (SweepResult :type "HitResult Structure (by ref)"))
  (bind _asvrpawn (cast `/Game/Blueprint/Player/VRPawn` OtherActor)
    (:`then`
      (if (`PrimitiveComponent.IsOverlappingActor` (`/Game/Blueprint/Player/VRPawn.CapsuleL` _asvrpawn) self)
        (set `self.HandInterract?` "NewEnumerator1")
        (elif (`PrimitiveComponent.IsOverlappingActor` (`/Game/Blueprint/Player/VRPawn.CapsuleR` _asvrpawn) self)
          (set `self.HandInterract?` "NewEnumerator2")
          (else
            (set `self.HandInterract?` "NewEnumerator0"))))
      (`/Game/Blueprint/Player/VRPawn.DeactiveInteractionMode` _asvrpawn)
      (bind _arms (`/Game/Blueprint/Player/VRPawn.Arms` _asvrpawn))
      (set `self.PreviousLocation` (- (`self.K2_GetActorLocation`) (`SceneComponent.GetSocketLocation` _arms (select `/Game/Blueprint/MainMenu/E_HandInterract` (`self.HandInterract?`) :`NewEnumerator1` "IndexL" :`NewEnumerator2` "IndexR" :!type "Name"))))
      (set `self.Arms` _arms))
    (:`CastFailed`
      (set `self.HandInterract?` "NewEnumerator0"))))

(event `self.Box.OnComponentEndOverlap`
  (params (OverlappedComponent :type "PrimitiveComponent Object Reference") (OtherActor :type "Actor Object Reference") (OtherComp :type "PrimitiveComponent Object Reference") (OtherBodyIndex :type Integer))
  (bind _returnvalue (`KismetArrayLibrary.Array_LastIndex` (`self.MapsMeshes`)))
  (bind _returnvalue_2 (+ (`self.MapIndex`) (`self.HandDirection`)))
  (bind _asvrpawn (cast `/Game/Blueprint/Player/VRPawn` OtherActor))
  (if (or (and (not (`/Game/Blueprint/Player/VRPawn.IndexLeft` _asvrpawn)) (`/Game/Blueprint/Player/VRPawn.CurlLeft` _asvrpawn) (`|EnumEquality` (`self.HandInterract?`) "NewEnumerator1")) (and (not (`/Game/Blueprint/Player/VRPawn.IndexRight` _asvrpawn)) (`/Game/Blueprint/Player/VRPawn.CurlRight` _asvrpawn) (`|EnumEquality` (`self.HandInterract?`) "NewEnumerator2")))
    (set `self.HandDirection` (`KismetMathLibrary.FTrunc` (`KismetMathLibrary.SignOfFloat` (`KismetMathLibrary.Dot_VectorVector` (- (- (`self.K2_GetActorLocation`) (`SceneComponent.GetSocketLocation` (`self.Arms`) (select `/Game/Blueprint/MainMenu/E_HandInterract` (`self.HandInterract?`) :`NewEnumerator1` "IndexL" :`NewEnumerator2` "IndexR" :!type "Name"))) (`self.PreviousLocation`)) (`SceneComponent.GetRightVector` (`self.Box`))))))
    (set `self.MapIndex` (`KismetMathLibrary.SelectInt` 0 (`KismetMathLibrary.SelectInt` _returnvalue _returnvalue_2 (< _returnvalue_2 0)) (> _returnvalue_2 _returnvalue)))
    (set `self.HandInterract?` "NewEnumerator0")
    (set `self.PreviousLocation` (0.0 0.0 0.0))))

(fn `UserConstructionScript`
  (bind _array (`|MakeArray` (`self.bleu`) (`self.violet`) (`self.rouge`) (`self.cyan`) (`self.jaune`)))
  (bind _output_get (set `self.MapsMeshes` _array))
  (for (_array_element _array_index) _output_get
    (bind _returnvalue (`PrimitiveComponent.CreateDynamicMaterialInstance` _array_element 0 "/Game/Materials/MenuChoose/M_SphereColor.M_SphereColor" "None"))
    (`MaterialInstanceDynamic.SetVectorParameterValue` _returnvalue "Color" (select `int` _array_index :`0` (struct :`R` 1.0 :`A` 1.0) :`1` (struct :`R` 0.510729 :`G` 1.0 :`A` 1.0) :`2` (struct :`G` 0.965735 :`B` 1.0 :`A` 1.0) :`3` (struct :`G` 0.016063 :`B` 1.0 :`A` 1.0) :`4` (struct :`R` 0.905564 :`B` 1.0 :`A` 1.0) :!type "LinearColor Structure"))
    (`PrimitiveComponent.SetMaterial` _array_element 0 _returnvalue)
    (`SceneComponent.K2_SetWorldLocation` _array_element (`SplineComponent.GetLocationAtTime` (`self.Spline`) (/ (* 1.0 _array_index) (`KismetArrayLibrary.Array_Length` _array)) "World" false) false false)))