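; BP_SplineTool_Orig is a spline placement tool that repeats one chosen mesh along a spline as instanced static mesh instances.
; Its construction script derives spacing from the mesh's X bounds plus an adjustable offset, then floors spline length over spacing for the count.
; Each instance sits at its distance along the spline in local space, oriented toward the next point and scaled by a rotation multiplier.
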(fn `GetLocationAtIndex`
  (params (A :type Integer))
  (returns (ReturnValue :type "Vector Structure"))
  (return (`SplineComponent.GetLocationAtDistanceAlongSpline` (`self.Spline`) (* A (`self.MeshSpacing`)) "Local")))

(fn `UserConstructionScript`
  (locals (NumberOfInstances :type Integer :default 0))
  (bind (_min _max) (break `Box` (`StaticMesh.GetBoundingBox` (`self.PlacedMesh`))))
  (`StaticMeshComponent.SetStaticMesh` (`self.InstancedStaticMesh`) (`self.PlacedMesh`))
  (bind _output_get (set `self.MeshSpacing` (+ (.x (- _max _min)) (`self.MeshOffset`))))
  (bind _output_get_2 (set `local.NumberOfInstances` (`KismetMathLibrary.FFloor` (/ (`SplineComponent.GetSplineLength` (`self.Spline`)) _output_get))))
  (for _index (range (+ _output_get_2 1))
    (bind _returnvalue (`self.GetLocationAtIndex` _index))
    (`InstancedStaticMeshComponent.AddInstance` (`self.InstancedStaticMesh`) (`KismetMathLibrary.MakeTransform` _returnvalue (* (`KismetMathLibrary.MakeRotFromX` (- (`self.GetLocationAtIndex` (+ _index 1)) _returnvalue)) (`self.MeshRotationMultiplier`))))))