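; Spline road tool that lines a spline with meshes picked randomly from PlacedMesh.
; The construction script derives spacing from one random pick's X bounds plus MeshOffset, then adds static mesh components along the spline, each aimed at the next point.
; BakeOutMeshes replaces those components with standalone StaticMeshActors at the same transforms.
; Instanced-mesh variants remain disconnected, and a debug print runs per placed mesh.
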(event `Bake Out Meshes`
  (for _array_element (`self.AllCreatedStaticMeshes`)
    (bind _returnvalue (`|SpawnActorFromClass` "/Script/Engine.StaticMeshActor" (`SceneComponent.K2_GetComponentToWorld` _array_element) "Undefined" "OverrideRootScale" null null))
    (`StaticMeshComponent.SetStaticMesh` (`StaticMeshActor.StaticMeshComponent` _returnvalue) (`StaticMeshComponent.StaticMesh` _array_element))
    (`ActorComponent.K2_DestroyComponent` _array_element)))

(fn `GetLocationAtIndex`
  (params (A :type Integer))
  (returns (ReturnValue :type "Vector Structure"))
  (return (`SplineComponent.GetLocationAtDistanceAlongSpline` (`self.Spline`) (* A (`self.MeshSpacing`)) "Local")))

(fn `UserConstructionScript`
  (locals (NumberOfInstances :type Integer :default 0) (CreatedStaticMesh :type "StaticMeshComponent Object Reference"))
  (bind (_outitem _outindex) (`KismetArrayLibrary.Array_Random` (`self.PlacedMesh`)))
  (bind (_min _max) (break `Box` (`StaticMesh.GetBoundingBox` _outitem)))
  (bind _x (.x (- _max _min)))
  (bind _output_get (set `self.MeshSpacing` (+ _x (`self.MeshOffset`))))
  (bind _output_get_2 (set `local.NumberOfInstances` (`KismetMathLibrary.FFloor` (/ (`SplineComponent.GetSplineLength` (`self.Spline`)) _output_get))))
  (for _index (range (+ _output_get_2 1))
    (bind _returnvalue (`self.GetLocationAtIndex` _index))
    (bind _returnvalue_2 (`AddComponent|NODE_AddStaticMeshComponent-3` :`RelativeTransform` (`KismetMathLibrary.MakeTransform` _returnvalue (* (`KismetMathLibrary.MakeRotFromX` (- (`self.GetLocationAtIndex` (+ _index 1)) _returnvalue)) (`self.MeshRotationMultiplier`)))))
    (bind _output_get_3 (set `local.CreatedStaticMesh` _returnvalue_2))
    (`KismetArrayLibrary.Array_Add` (`self.AllCreatedStaticMeshes`) _output_get_3)
    (`StaticMeshComponent.SetStaticMesh` _returnvalue_2 _outitem)
    (`KismetSystemLibrary.PrintString` (`KismetStringLibrary.Concat_StrStr` (`KismetStringLibrary.Conv_IntToString` _outindex) "            " (`KismetSystemLibrary.GetDisplayName` _outitem) "                                           " (`KismetStringLibrary.Conv_DoubleToString` _x)))))