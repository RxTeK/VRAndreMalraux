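; Spline placement tool that builds a chain of bendable spline mesh components along its spline.
; The construction script adds one component per segment, fitting its start and end to neighboring points' locations and tangents.
; BakeOutMeshes replaces the tracked components with StaticMeshActors, copying only mesh and transform, not spline deformation.
; Disconnected leftover logic places random meshes at bounds-based spacing and never runs.
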(event `Bake Out Meshes`
  (for _array_element (`self.AllCreatedStaticMeshes`)
    (bind _returnvalue (`|SpawnActorFromClass` "/Script/Engine.StaticMeshActor" (`SceneComponent.K2_GetComponentToWorld` _array_element) "Undefined" "OverrideRootScale" null null))
    (`StaticMeshComponent.SetStaticMesh` (`StaticMeshActor.StaticMeshComponent` _returnvalue) (`StaticMeshComponent.StaticMesh` _array_element))
    (`ActorComponent.K2_DestroyComponent` _array_element)))

(fn `GetLocationAtIndex`
  (params (A :type Integer))
  (returns (ReturnValue :type "Vector Structure"))
  (return (`SplineComponent.GetLocationAtDistanceAlongSpline` (`self.Spline`) (* A (`self.MeshSpacing`)) "Local")))

(fn `UserConstructionScript`
  (locals (NumberOfInstances :type Integer :default 0) (CreatedStaticMesh :type "StaticMeshComponent Object Reference"))
  (bind _spline (`self.Spline`))
  (for _index (range (+ (- (`SplineComponent.GetNumberOfSplinePoints` (`self.Spline`)) 2) 1))
    (bind _returnvalue (`AddComponent|NODE_AddSplineMeshComponent-3`))
    (bind _output_get (set `local.CreatedStaticMesh` _returnvalue))
    (`KismetArrayLibrary.Array_Add` (`self.AllCreatedStaticMeshes`) _output_get)
    (bind (_location _tangent) (`SplineComponent.GetLocationAndTangentAtSplinePoint` _spline _index "Local"))
    (bind (_location_2 _tangent_2) (`SplineComponent.GetLocationAndTangentAtSplinePoint` _spline (+ _index 1) "Local"))
    (`SplineMeshComponent.SetStartAndEnd` _returnvalue _location _tangent _location_2 _tangent_2 true)
    (`SceneComponent.K2_AttachToComponent` _returnvalue (`self.DefaultSceneRoot`) "None" "KeepRelative" "KeepRelative" "KeepRelative" true)))